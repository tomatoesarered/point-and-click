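; BP_Button is an interactable button that alternately opens and closes a door on each Interact event.
; On BeginPlay it caches the first BP_Door found in the level, and a FlipFlop switches between its OpenDoor and CloseDoor calls.
; When an override camera length is set, it also calls CamOverride on the player character with a transform and a stop time computed from the current UTC Unix timestamp.
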(event `self.ReceiveBeginPlay`
  (bind _returnvalue (`GameplayStatics.GetActorOfClass` "/Game/Platform/BP_Door.BP_Door_C"))
  (set `self.NewVar` _returnvalue))

(event `/Game/Platform/BPI_Interact.Interact`
  (bind _newvar (`self.NewVar`))
  (bind _overridecamlength (`self.OverrideCamLength`))
  (`/Engine/EditorBlueprintResources/StandardMacros.FlipFlop`
    (:`A`
      (`/Game/Platform/BP_Door.Open Door` _newvar))
    (:`B`
      (`/Game/Platform/BP_Door.Close Door` _newvar)))
  (if (> _overridecamlength 0.0)
    (bind _asbp_char_pand_c (cast `/Game/Player/BP_CharPandC` (`GameplayStatics.GetPlayerPawn` 0)))
    (`/Game/Player/BP_CharPandC.CamOverride` _asbp_char_pand_c (`self.OverrideCamTransform`) (+ _overridecamlength (`KismetMathLibrary.ToUnixTimestampDouble` (`KismetMathLibrary.UtcNow`))))))

(fn `UserConstructionScript`)