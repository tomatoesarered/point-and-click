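; BP_SplineObject is an actor that travels along the spline of a referenced SplineToFollow actor, starting at BeginPlay.
; MoveObject plays a timeline at a rate of one over TimeToComplete, so that variable scales the trip's duration.
; Each update maps the timeline track to a distance along the spline and sets the actor's world location and rotation from that point.
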(event `self.ReceiveBeginPlay`
  (`self.MoveObject`))

(event `MoveObject`
  (bind _spline (`/Game/Platform/Spline/BP_Splinepath.Spline` (`self.SplineToFollow`)))
  (`TimelineComponent.SetPlayRate` (`self.TL_Move`) (/ 1.0 (`self.TimeToComplete`)))
  (bind (_direction _movetrack) (`Timeline|TL_Move`)
    (:`Update`
      (bind _returnvalue (`KismetMathLibrary.Lerp` 0.0 (`SplineComponent.GetSplineLength` _spline) _movetrack))
      (`self.K2_SetActorLocationAndRotation` (`SplineComponent.GetLocationAtDistanceAlongSpline` _spline _returnvalue "World") (`SplineComponent.GetRotationAtDistanceAlongSpline` _spline _returnvalue "World")))))

(fn `UserConstructionScript`)