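; BP_CharPandC is a point-and-click player character with an angled spring-arm camera, visible cursor and health widget.
; Left click traces under the cursor, spawns a location marker and uses SimpleMoveToLocation to walk there.
; E sphere-traces nearby WorldDynamic objects and messages those implementing BPI_Interact.
; The timed camera override is unfinished, with its transform nodes unwired, and the health-bar update only attempts to set zero percent.
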(event `CamOverrideTick`
  (if (< (`KismetMathLibrary.ToUnixTimestampDouble` (`KismetMathLibrary.UtcNow`)) (`self.TimeStopCam`))
    (bind _returnvalue (`BlueprintCameraPoseFunctionLibrary.MakeCameraPoseFromCameraComponent` (`self.Camera`)))))

(event `Show Mouse Cursor`
  ; Show mouse cursor
  (set `PlayerController.bShowMouseCursor` true (`GameplayStatics.GetPlayerController` 0)))

(event `CamOverride`
  (params (Position :type "Transform Structure") (TickStop :type "Float (double-precision)"))
  (if (< (`KismetMathLibrary.ToUnixTimestampDouble` (`KismetMathLibrary.UtcNow`)) TickStop)
    (set `self.TimeStopCam` TickStop)
    (set `self.TransformCam` Position)))

(event `self.ReceiveBeginPlay`
  (`self.Show Mouse Cursor`)
  (`SceneComponent.K2_SetWorldRotation` (`self.SpringArm`) (struct :`Pitch` -45.0 :`Yaw` -45.0) false false)
  (bind _returnvalue (`|CreateWidget` "/Game/UI/BP_Health.BP_Health_C"))
  (`UserWidget.AddToPlayerScreen` _returnvalue 0)
  (set `self.HealthWidget` _returnvalue))

(event `UpdateHealthBar`
  (bind _asprogress_bar (cast `ProgressBar` (`self.HealthWidget`)))
  (`ProgressBar.SetPercent` _asprogress_bar 0.0))

(event `self.ReceiveTick`
  (params (DeltaSeconds :type "Float (single-precision)"))
  (`self.CamOverrideTick`))

(event `Character Movement`
  (bind (_worldlocation _worlddirection) (`PlayerController.DeprojectMousePositionToWorld` (`GameplayStatics.GetPlayerController` 0)))
  (bind _outhit (`KismetSystemLibrary.LineTraceSingle` _worldlocation (+ _worldlocation (* _worlddirection 50000)) "TraceTypeQuery1"))
  (bind (_bblockinghit _binitialoverlap _time _distance _location) (`GameplayStatics.BreakHitResult` _outhit))
  (if _bblockinghit
    (`|SpawnActorFromClass` "/Game/Player/BP_LocationPoint.BP_LocationPoint_C" (`KismetMathLibrary.MakeTransform` (`KismetMathLibrary.MakeVector` (.x _location) (.y _location) 2.0)) "Undefined" "MultiplyWithRoot" null null)
    (`AIBlueprintHelperLibrary.SimpleMoveToLocation` (`GameplayStatics.GetPlayerController` 0) _location)))

(event `Key|LeftMouseButton`
  (params (Key :type "Key Structure"))
  (:`Pressed`
    (`self.Character Movement`)))

(event `Key|E`
  (params (Key :type "Key Structure"))
  (bind _returnvalue (`self.K2_GetActorLocation`))
  (:`Pressed`
    (bind (_outhits _returnvalue_2) (`KismetSystemLibrary.SphereTraceMultiForObjects` _returnvalue _returnvalue 150.0 (`|MakeArray` "ObjectTypeQuery2" :!type "EObjectTypeQuery Enum")))
    (if _returnvalue_2
      (for _array_element _outhits
        (bind (_bblockinghit _binitialoverlap _time _distance _location _impactpoint _normal _impactnormal _physmat _hitactor) (`GameplayStatics.BreakHitResult` _array_element))
        (if (`KismetSystemLibrary.DoesImplementInterface` _hitactor "/Game/Platform/BPI_Interact.BPI_Interact_C")
          (message `/Game/Platform/BPI_Interact.Interact` _hitactor))))))

(fn `UserConstructionScript`)