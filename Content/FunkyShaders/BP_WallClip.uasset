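; BP_WallClip is a wall actor that feeds the player's position to a clipping shader.
; On BeginPlay it creates a dynamic instance of the Clipping material on its Cube and caches the first player pawn.
; Every Tick it writes that pawn's world location into the material's PlayerPosition vector parameter, leaving any visual clipping to the material.
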(event `self.ReceiveBeginPlay`
  (bind _returnvalue (`PrimitiveComponent.CreateDynamicMaterialInstance` (`self.Cube`) 0 "/Game/FunkyShaders/Clipping.Clipping" "None"))
  (set `self.DynamicMaterial` _returnvalue)
  (set `self.ThatThing` (`GameplayStatics.GetPlayerPawn` 0)))

(event `self.ReceiveTick`
  (params (DeltaSeconds :type "Float (single-precision)"))
  (`MaterialInstanceDynamic.SetVectorParameterValue` (`self.DynamicMaterial`) "PlayerPosition" (`KismetMathLibrary.Conv_VectorToLinearColor` (`self.K2_GetActorLocation` (`self.ThatThing`)))))

(fn `UserConstructionScript`)